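; Unit Blueprint in the Advanced Turn Based Tile Toolkit that derives Fire Emblem-style combat stats from base attributes.
; Accuracy sums Skill, half of Luck and weapon accuracy, while Avoid sums half of Luck and Speed.
; The same formulas run in both the Construction Script and BeginPlay, with no recalculation afterwards in this Blueprint.
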(event `self.ReceiveBeginPlay`
  (bind _returnvalue (/ (`self.Luck`) 2.0))
  (set `self.UnitAccuracy` (+ (`self.Skill`) _returnvalue (`self.WeaponAccuracy`)))
  (set `self.UnitAvoid` (+ _returnvalue (`self.Speed`))))

(fn `ConstructionScript`
  (bind _returnvalue (/ (`self.Luck`) 2.0))
  (set `self.UnitAccuracy` (+ (`self.Skill`) _returnvalue (`self.WeaponAccuracy`)))
  (set `self.UnitAvoid` (+ _returnvalue (`self.Speed`))))